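; BP_ClassOneActor is an actor that demonstrates basic Blueprint debugging, effect spawning and movement on BeginPlay.
; It prints two screen messages, draws a debug sphere and cylinder at a hardcoded world position, and spawns a P_Fire emitter there.
; Timed delays then step the spawned emitter twice along +Y and finally shift the StaticMesh component along -Y, all without sweep.
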(event EventBeginPlay
  (Development|PrintString "Hello" true true "(R=0.000000,G=0.660000,B=1.000000,A=1.000000)" 1e+01)
  (Development|PrintString "World" true true "(R=1.000000,G=0.077328,B=0.463597,A=1.000000)" 1e+01)
  (Rendering|Debug|DrawDebugSphere "1530.000000,1010.000000,20.000000" 2e+02 12 "(R=0.346674,G=0.261674,B=1.000000,A=1.000000)" 3e+01 2.0)
  (Class|KismetSystemLibrary|DrawDebugCylinder "1530.000000,1010.000000,20.000000" "1530.000000,1010.000000,200.000000" 1e+02 12 "(R=1.000000,G=1.000000,B=1.000000,A=1.000000)" 3e+01 2.0)
  (bind _returnvalue (Effects|SpawnEmitteratLocation "/Game/StarterContent/Particles/P_Fire.P_Fire" "1530.000000,1010.000000,20.000000"))
  (Utilities|FlowControl|Delay 2.0)
  (Transformation|AddWorldOffset _returnvalue "0.000000,200.000000,0.000000" false false)
  (Utilities|FlowControl|Delay 2.0)
  (Transformation|AddWorldOffset _returnvalue "0.000000,200.000000,0.000000" false false)
  (Utilities|FlowControl|Delay 1.0)
  (Transformation|AddWorldOffset (Variables|Default|GetStaticMesh) "0.000000,-200.000000,0.000000" false false))

(fn ConstructionScript)