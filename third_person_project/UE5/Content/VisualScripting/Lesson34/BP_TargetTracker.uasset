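; BP_TargetTracker is a lesson Blueprint for finding where a target actor lies relative to an owner actor using vector math.
; Tick stores the normalized direction from OwnerActor to TargetActor in DirectionVector.
; Unconnected, never-run chains would print the angle to the target via dot product and acos, and test left or right via the sign of the cross product's Z.
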(event EventBeginPlay)

(event Collision|EventActorBeginOverlap
  (params (OtherActor :type Actor%20Object%20Reference)))

(event EventTick
  (params (DeltaSeconds :type Float%20%28single-precision%29))
  (bind _output_get (Variables|Default|SetDirectionVector (Math|Vector|Normalize (- (Transformation|GetActorLocation (Variables|Default|GetTargetActor)) (Transformation|GetActorLocation (Variables|Default|GetOwnerActor)))))))

(fn ConstructionScript)