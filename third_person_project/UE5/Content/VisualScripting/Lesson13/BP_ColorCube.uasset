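; BP_ColorCube is an interactable cube whose color the player picks with a UI slider.
; Its box overlap shows a press-E prompt for the player character and enables E to toggle the color widget and mouse cursor.
; Leaving the box hides both widgets and the cursor.
; Tick maps the slider value to hue at full saturation and brightness, writing it to a dynamic material created in the Construction Script.
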(event OnComponentBeginOverlap(Box)
  (params (OverlappedComponent :type Primitive%20Component%20Object%20Reference) (OtherActor :type Actor%20Object%20Reference) (OtherComp :type Primitive%20Component%20Object%20Reference) (OtherBodyIndex :type Integer) (bFromSweep :type Boolean) (SweepResult :type Hit%20Result%20Structure%20%28by%20ref%29))
  ;[1 1 1] Interact Promt Press E (Colission Box)
  (if (== OtherActor (Game|GetPlayerCharacter 0))
    (Variables|Default|SetCanChangeColor true)
    (UserInterface|Viewport|AddtoViewport (Variables|Default|GetInteractPromt) 0)))

(event OnComponentEndOverlap(Box)
  (params (OverlappedComponent :type Primitive%20Component%20Object%20Reference) (OtherActor :type Actor%20Object%20Reference) (OtherComp :type Primitive%20Component%20Object%20Reference) (OtherBodyIndex :type Integer))
  ;[1 1 1] Interact Promt Press E (Colission Box)
  (if (== (Game|GetPlayerCharacter 0) OtherActor)
    (Variables|Default|SetCanChangeColor false)
    (Widget|RemovefromParent (Variables|Default|GetInteractPromt))
    (Widget|SetVisibility (Variables|Default|GetWidget_0) "Hidden")
    (Variables|/Script/Engine.PlayerController|SetbShowMouseCursor (Game|GetPlayerController 0) false)))

(event EventBeginPlay
  (bind _returnvalue (Game|GetPlayerController 0))
  (Utilities|FlowControl|Sequence
    (:then_0
      ;[1 1 1] WBP PRESS E TO INTERACT
      (bind _returnvalue_2 (UserInterface|CreateWidget "/Game/VisualScripting/Lesson13/WBP_E_Interact.WBP_E_Interact_C" (Game|GetPlayerController 0)))
      (Variables|Default|SetInteractPromt _returnvalue_2))
    (:then_1
      ;[1 1 1] WBP COLOR
      (Input|EnableInput _returnvalue)
      (bind _returnvalue_3 (UserInterface|CreateWidget "/Game/VisualScripting/Lesson13/WBP_UIColor.WBP_UIColor_C" _returnvalue))
      (Variables|Default|SetWidget_0 _returnvalue_3)
      (UserInterface|Viewport|AddtoViewport (Variables|Default|GetWidget_0) 0)
      (Widget|SetVisibility (Variables|Default|GetWidget_0) "Hidden"))))

(event Collision|EventActorBeginOverlap
  (params (OtherActor :type Actor%20Object%20Reference)))

(event EventTick
  (params (DeltaSeconds :type Float%20%28single-precision%29))
  ;[1 1 1] RGB Color Palette
  (Rendering|Material|SetVectorParameterValue (Variables|Default|GetDynamicMaterial) "Color" (Class|KismetMathLibrary|HSVtoRGB (Math|Float|MapRangeClamped (Class|Slider|GetValue (Variables|/Game/VisualScripting/Lesson13/WBP_UIColor.WBP_UIColor_C|GetSlider_158 (Variables|Default|GetWidget_0))) 0.0 1.0 0.0 359.0) 1.0 1.0 1.0) :!class /Script/Engine.MaterialInstanceDynamic))

(event Input|KeyboardEvents|E
  (params (Key :type Key%20Structure :default "None"))
  (bind _returnvalue (Game|GetPlayerController 0))
  (bind _widget_0 (Variables|Default|GetWidget_0))
  (:Pressed
    ;[1 1 1] E Interaction
    (if (Variables|Default|GetCanChangeColor)
      (Utilities|FlowControl|FlipFlop
        (:A
          (Widget|SetVisibility _widget_0 "Visible")
          (Input|SetInputModeGameandUI _returnvalue 0 "DoNotLock" true false)
          (Variables|/Script/Engine.PlayerController|SetbShowMouseCursor _returnvalue true))
        (:B
          (Widget|SetVisibility _widget_0 "Hidden")
          (Variables|/Script/Engine.PlayerController|SetbShowMouseCursor _returnvalue false))))))

(fn ConstructionScript
  (bind _returnvalue (Rendering|Material|CreateDynamicMaterialInstance (Variables|Default|GetCube) 0 "/Game/VisualScripting/Lesson13/M_ColorCube.M_ColorCube" "None" :!class /Script/Engine.PrimitiveComponent))
  (Variables|Default|SetDynamicMaterial _returnvalue))