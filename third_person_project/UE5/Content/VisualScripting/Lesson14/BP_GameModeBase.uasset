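; Game mode Blueprint that keeps interactable actors informed of how many of them are in the level.
; On BeginPlay it starts a looping one-second timer that resets and recounts all actors implementing BPI_GetInteractableObjectsUpdated.
; It then sends the total to each of those actors through an interface message, so no casts to specific classes are needed.
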(event Custom|TimerEventInteractable
  (Variables|Default|SetInteractebleObjectsNum 0)
  (bind _outactors (Actor|GetAllActorswithInterface "/Game/VisualScripting/Lesson14/BPI_GetInteractableObjectsUpdated.BPI_GetInteractableObjectsUpdated_C"))
  (for _array_element _outactors
    (bind _result (Math|Integer|IncrementInt (Variables|Default|GetInteractebleObjectsNum))
      (:%20%20
        (Variables|Default|SetInteractebleObjectsNum _result))))
  (bind _outactors_2 (Actor|GetAllActorswithInterface "/Game/VisualScripting/Lesson14/BPI_GetInteractableObjectsUpdated.BPI_GetInteractableObjectsUpdated_C"))
  (for _array_element_2 _outactors_2
    (Class|BPIGetInteractableObjectsUpdated|OnInteracteblesInfoUpdated(Message) _array_element_2 (Variables|Default|GetInteractebleObjectsNum))))

(event EventBeginPlay
  (Utilities|Time|SetTimerbyEvent (delegate Custom|TimerEventInteractable) 1.0 true))

(event EventTick
  (params (DeltaSeconds :type Float%20%28single-precision%29)))

(fn ConstructionScript)