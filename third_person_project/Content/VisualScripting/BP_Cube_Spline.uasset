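; BP_Cube_Spline is a Blueprint that moves a Cube component along a Spline.
; Each Tick advances a distance by a tenth of SpeedOnSpine, independent of delta time, so speed varies with frame rate.
; The Cube takes the spline's world transform at that distance, ignoring scale, without sweeping.
; When Loop is enabled, the distance resets to zero on reaching the spline's end.
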(event EventTick
  (params (DeltaSeconds :type Float%20%28single-precision%29))
  (bind _output_get (Variables|Default|SetPositionOnSpine (+ (* 0.1 (Variables|Default|GetSpeedOnSpine)) (Variables|Default|GetPositionOnSpine))))
  (Transformation|SetWorldTransform (Variables|Default|GetCube) (Spline|GetTransformatDistanceAlongSpline (Variables|Default|GetSpline) _output_get "World" false) false false)
  (if (Variables|Default|GetLoop)
    (if (>= (Variables|Default|GetPositionOnSpine) (Spline|GetSplineLength (Variables|Default|GetSpline)))
      (Variables|Default|SetPositionOnSpine 0.0))))

(fn ConstructionScript)