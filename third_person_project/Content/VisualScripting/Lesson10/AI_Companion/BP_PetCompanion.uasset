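; BP_PetCompanion is a wolf pet that follows the player and has bark, sit and play-dead events.
; From BeginPlay, FollowPlayer runs AI MoveTo toward the player and calls itself again on success only.
; The trick events play animations directly on the mesh, with delays before the looping sit and death animations.
; Sit and play dead also stop movement and zero walk speed, which nothing here restores.
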(event Custom|SitDown
  ;[1 1 1] PetIsSitting
  (AI|Navigation|StopMovement (Pawn|GetController))
  (Variables|/Script/Engine.CharacterMovementComponent|SetMaxWalkSpeed (Variables|Character|GetCharacterMovement) 0.0)
  (Components|Animation|PlayAnimation (Variables|Character|GetMesh) "/Game/AnimalVarietyPack/Wolf/Animations/ANIM_Wolf_GoToRest.ANIM_Wolf_GoToRest" false)
  (Utilities|FlowControl|Delay 1.0)
  (Components|Animation|PlayAnimation (Variables|Character|GetMesh) "/Game/AnimalVarietyPack/Wolf/Animations/ANIM_Wolf_Rest.ANIM_Wolf_Rest" true))

(event Custom|Bark
  ;[1 1 1] Bark
  (Components|Animation|PlayAnimation (Variables|Character|GetMesh) "/Game/AnimalVarietyPack/Wolf/Animations/ANIM_Wolf_Howl.ANIM_Wolf_Howl" true))

(event Custom|PlayDead
  ;[1 1 1] PlayDead
  (AI|Navigation|StopMovement (Pawn|GetController))
  (Variables|Default|SetIsPlayingDeath true)
  (Variables|/Script/Engine.CharacterMovementComponent|SetMaxWalkSpeed (Variables|Character|GetCharacterMovement) 0.0)
  (Components|Animation|PlayAnimation (Variables|Character|GetMesh) "/Game/AnimalVarietyPack/Wolf/Animations/ANIM_Wolf_Death.ANIM_Wolf_Death" false)
  (Utilities|FlowControl|Delay 5.0)
  (Components|Animation|PlayAnimation (Variables|Character|GetMesh) "/Game/AnimalVarietyPack/Wolf/Animations/ANIM_Wolf_Death.ANIM_Wolf_Death" true))

(event Custom|FollowPlayer
  ;[1 1 1] Lesson10 FollowPlayer
  (AI|AIMoveTo self "0, 0, 0" (Game|GetPlayerCharacter 0) 2e+02 false
    (:OnSuccess
      (CallFunction|FollowPlayer))))

(event EventBeginPlay
  ;[1 1 1] PetIsSitting
  (CallFunction|FollowPlayer)
  (if (not (or (Variables|Default|GetIsSitting) (Variables|Default|GetIsPlayingDeath)))
    _))

(fn ConstructionScript)