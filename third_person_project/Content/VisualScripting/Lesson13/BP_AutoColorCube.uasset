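; Interactive cube actor that recolors itself when the player presses E inside its trigger box.
; Box overlap with the player enables the action and shows an E prompt widget; leaving removes it and resets the color to black.
; ChangeColor sets a dynamic material's Color parameter through HSVToRGB with a random 0–1 hue, which stays near red because that node expects degrees.
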(event OnComponentBeginOverlap(Box)
  (params (OverlappedComponent :type Primitive%20Component%20Object%20Reference) (OtherActor :type Actor%20Object%20Reference) (OtherComp :type Primitive%20Component%20Object%20Reference) (OtherBodyIndex :type Integer) (bFromSweep :type Boolean) (SweepResult :type Hit%20Result%20Structure%20%28by%20ref%29))
  ;[1 1 1] Interact Promt Press E (Colission Box)
  (if (== OtherActor (Game|GetPlayerCharacter 0))
    (Variables|Default|SetCanChangeColor true)
    (bind _returnvalue (UserInterface|CreateWidget "/Game/VisualScripting/Lesson13/WBP_E_Interact.WBP_E_Interact_C" (Game|GetPlayerController 0)))
    (Variables|Default|SetInteractPromt _returnvalue)
    (UserInterface|Viewport|AddtoViewport (Variables|Default|GetInteractPromt) 0)))

(event OnComponentEndOverlap(Box)
  (params (OverlappedComponent :type Primitive%20Component%20Object%20Reference) (OtherActor :type Actor%20Object%20Reference) (OtherComp :type Primitive%20Component%20Object%20Reference) (OtherBodyIndex :type Integer))
  ;[1 1 1] Interact Promt Press E (Colission Box)
  (if (== (Game|GetPlayerCharacter 0) OtherActor)
    (Variables|Default|SetCanChangeColor false)
    (Rendering|Material|SetVectorParameterValue (Variables|Default|GetDynamicMaterial) "Color" "(R=0.000000,G=0.000000,B=0.000000,A=1.000000)" :!class /Script/Engine.MaterialInstanceDynamic)
    (bind _interactpromt (Variables|Default|GetInteractPromt)
      (:then
        (Widget|RemovefromParent _interactpromt))
      (:else))))

(event Collision|EventActorBeginOverlap
  (params (OtherActor :type Actor%20Object%20Reference)))

(event EventBeginPlay
  ;[1 1 1] Shows Dynamic Material
  (bind _returnvalue (Rendering|Material|CreateDynamicMaterialInstance (Variables|Default|GetCube) 0 0 "None" :!class /Script/Engine.PrimitiveComponent))
  (Variables|Default|SetDynamicMaterial _returnvalue)
  (Input|EnableInput (Game|GetPlayerController 0)))

(event Input|KeyboardEvents|E
  (params (Key :type Key%20Structure :default "None"))
  ;[1 1 1] E Pressed
  (:Pressed
    (if (Variables|Default|GetCanChangeColor)
      (CallFunction|ChangeColor))))

(fn ConstructionScript
  (bind _returnvalue (Rendering|Material|CreateDynamicMaterialInstance (Variables|Default|GetCube) 0 "/Game/VisualScripting/Lesson13/M_ColorCube.M_ColorCube" "None" :!class /Script/Engine.PrimitiveComponent))
  (Variables|Default|SetDynamicMaterial _returnvalue))

(fn ChangeColor
  (Rendering|Material|SetVectorParameterValue (Variables|Default|GetDynamicMaterial) "Color" (Class|KismetMathLibrary|HSVtoRGB (Math|Random|RandomFloatinRange 0.0 1.0) 1.0 1.0 0.0) :!class /Script/Engine.MaterialInstanceDynamic))