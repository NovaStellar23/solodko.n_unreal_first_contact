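; BP_MyHouse is an Actor Blueprint that builds a simple house at runtime and then rescales it in timed stages.
; BeginPlay adds static mesh components for a floor, walls including a window piece, and a pyramid roof.
; After each delay it sets the root's world scale from HouseScaleVector or HouseScale with growing multipliers.
; A disconnected chain of variable, math and print experiments never runs.
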(event EventBeginPlay
  (bind _housescale (Variables|Default|GetHouseScale))
  (bind _returnvalue (* _housescale 8.0))
  (Development|PrintString "Starting Construction")
  ;[1 1 1] Foundation
  (bind _returnvalue_2 (AddComponent|AddStaticMeshComponent false))
  (Components|StaticMesh|SetStaticMesh _returnvalue_2 "/Game/StarterContent/Architecture/Floor_400x400.Floor_400x400")
  (Transformation|SetRelativeLocation _returnvalue_2 "1.478141,-0.426644,9.880945" false false)
  (Transformation|SetRelativeScale3D _returnvalue_2 "0.500000,1.000000,0.500000")
  ;[1 1 1] Wall1
  (bind _returnvalue_3 (AddComponent|AddStaticMeshComponent false (Math|Transform|MakeTransform "0, 0, 0" "0, 0, 0" "0.500000,-1.000000,0.500000")))
  (Components|StaticMesh|SetStaticMesh _returnvalue_3 "/Game/StarterContent/Architecture/Wall_Window_400x300.Wall_Window_400x300")
  ;[1 1 1] Wall2
  (bind _returnvalue_4 (AddComponent|AddStaticMeshComponent false (Math|Transform|MakeTransform "-1.808288,814.201397,-5.602100" "0, 0, 0" "0.500000,-0.750000,0.500000")))
  (Components|StaticMesh|SetStaticMesh _returnvalue_4 "/Game/StarterContent/Architecture/Wall_400x300.Wall_400x300")
  ;[1 1 1] Wall3
  (bind _returnvalue_5 (AddComponent|AddStaticMeshComponent false (Math|Transform|MakeTransform "-1.808288,814.201397,-5.602100" "0.000000,89.999999,0.000000" "-0.250000,1.000000,0.500000")))
  (Components|StaticMesh|SetStaticMesh _returnvalue_5 "/Game/StarterContent/Architecture/Wall_400x300.Wall_400x300")
  ;[1 1 1] Wall4
  (bind _returnvalue_6 (AddComponent|AddStaticMeshComponent false (Math|Transform|MakeTransform "196.761490,812.479999,-2.281653" "0.000000,89.999999,0.000000" "-0.250000,1.000000,0.500000")))
  (Components|StaticMesh|SetStaticMesh _returnvalue_6 "/Game/StarterContent/Architecture/Wall_400x300.Wall_400x300")
  ;[1 1 1] Roof
  (bind _returnvalue_7 (AddComponent|AddStaticMeshComponent false (Math|Transform|MakeTransform "94.144657,444.809259,148.674464" "1.408380,-0.386651,-0.373060" "2.500000,10.250000,0.500000")))
  (Components|StaticMesh|SetStaticMesh _returnvalue_7 "/Game/StarterContent/Shapes/Shape_QuadPyramid.Shape_QuadPyramid")
  (Utilities|FlowControl|Delay (Variables|Default|GetDelayDuration))
  (Transformation|SetWorldScale3D (Variables|Default|GetDefaultSceneRoot) (Variables|Default|GetHouseScaleVector))
  (Utilities|FlowControl|Delay (Variables|Default|GetDelayDuration))
  (Transformation|SetWorldScale3D (Variables|Default|GetDefaultSceneRoot) (* (Variables|Default|GetHouseScaleVector) "4.000000,4.000000,4.000000"))
  (Utilities|FlowControl|Delay (Variables|Default|GetDelayDuration))
  (Transformation|SetWorldScale3D (Variables|Default|GetDefaultSceneRoot) (Math|Vector|MakeVector _returnvalue _returnvalue _returnvalue)))

(fn ConstructionScript)